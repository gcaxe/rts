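; PC_map1 is the player controller for map1, turning left mouse input into drawing on the HUD's move-pawn widget.
; On BeginPlay it casts the game mode's HUD class to HUD_map1 and caches the matching actor found in the world.
; Pressing the left button enables CanDraw on that HUD's UWMovepawn, and releasing disables it and resets the widget.
; A local-controller check exists but is disconnected and never runs.
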(event `self.ReceiveBeginPlay`
  (bind _ashud_map_1 (castclass `/Game/Mythings/BP/UI/HUD_map1` (`GameModeBase.HUDClass` (`GameplayStatics.GetGameMode`))))
  (bind _returnvalue (`GameplayStatics.GetActorOfClass` _ashud_map_1))
  (set `self.HUD_map1` _returnvalue))

(event `Key|LeftMouseButton`
  (params (Key :type "Key Structure"))
  (bind _uw_movepawn (`/Game/Mythings/BP/UI/HUD_map1.UW_movepawn` (`self.HUD_map1`)))
  (:`Pressed`
    (set `/Game/Mythings/BP/UI/UW_movepawn.CanDraw` true _uw_movepawn))
  (:`Released`
    (set `/Game/Mythings/BP/UI/UW_movepawn.CanDraw` false _uw_movepawn)
    (`/Game/Mythings/BP/UI/UW_movepawn.reset` _uw_movepawn)))

(fn `UserConstructionScript`)